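; A mini-game pressure button actor that sinks while any actor overlaps its Box.
; Each Tick steps Button's height down by a fixed, frame-rate-dependent amount through a near-instant MoveComponentTo, clamped between zero and ButtonOffSet.
; The no-overlap branch computes the matching upward step, but its move has no component wired.
; The construction script sizes an Arrow to ButtonOffSet to show the travel distance.
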(event Collision|EventActorBeginOverlap
  (params (OtherActor :type Actor%20Object%20Reference)))

(event EventTick
  (params (DeltaSeconds :type Float%20%28single-precision%29))
  (bind _button (Variables|Default|GetButton))
  (if (> (Utilities|Array|Length (Collision|GetOverlappingActors (Variables|Default|GetBox) 0 :!class /Script/Engine.PrimitiveComponent)) 0)
    (Components|MoveComponentTo _button (Math|Vector|MakeVector 0.0 0.0 (Math|Float|Clamp(Float) (- (.z (Variables|/Script/Engine.SceneComponent|GetRelativeLocation _button)) 3.0) 0.0 (Variables|Default|GetButtonOffSet))) "0, 0, 0" false false 0.0001 false)
    (else
      (Components|MoveComponentTo 0 (Math|Vector|MakeVector 0.0 0.0 (Math|Float|Clamp(Float) (+ (.z (Variables|/Script/Engine.SceneComponent|GetRelativeLocation (Variables|Default|GetButton))) 3.0) 0.0 (Variables|Default|GetButtonOffSet))) "0, 0, 0" false false 0.0001 false))))

(fn ConstructionScript
  (Variables|/Script/Engine.ArrowComponent|SetArrowLength (Variables|Default|GetArrow) (Variables|Default|GetButtonOffSet)))